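; Destructible static mesh actor that breaks Pivot Painter elements along weapon rays or around supplied hit points.
; Construction binds the origin/extent texture and UAV render targets for timestamps and normal/random data to dynamic materials.
; With SphereCollisionFeedback, BeginPlay reads that texture to spawn pawn-blocking spheres per element.
; Asynchronous destroy calls receive both targets and return indices for sphere removal; ray hits also report hit or miss to the weapon.
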(event Custom|SphereHit
  (params (Ray%20Origin :type Vector%20%28by%20ref%29) (Ray%20End :type Vector%20%28by%20ref%29) (Spread%20Distance :type Float%20%28double-precision%29) (Max%20Delay :type Float%20%28double-precision%29) (Input%20Hit%20Point :type Vector))
  ;[0 1 0.7788] Sphere Hit
  (bind _outstruct (|ExecutePivotPainterDestroybyHit Ray%20Origin Ray%20End Spread%20Distance Max%20Delay (Math|Transform|ToMatrix(Transform) (Transformation|GetWorldTransform (Variables|Default|GetStaticMesh))) (Variables|PivotPainterInputs|GetOrigin_Extent) (Variables|Textures|GetTimestamp) (Variables|Textures|GetNormal%20Random) (Utilities|Time|GetTimeSeconds) Input%20Hit%20Point)
    (:Completed
      (Utilities|DisableSphereCollisionatIndex (.Count (Utilities|Struct|BreakOutStruct _outstruct)) (.OutIndexes (Utilities|Struct|BreakOutStruct _outstruct))))))

(event Custom|RayHitEvent
  (params (Ray%20Origin :type Vector) (Ray%20End :type Vector) (Spread%20Distance :type Float%20%28double-precision%29) (MaxDelay :type Float%20%28double-precision%29) (WeaponReference :type BP%20Weapon%20Component%20Object%20Reference%20%28by%20ref%29))
  ;[0.08369 0.3071 1] First Ray Hit
  (if (not (Variables|Default|GetIsWorking))
    (bind _outstruct (|ExecutePivotPainterDestroy Ray%20Origin Ray%20End Spread%20Distance MaxDelay (Math|Transform|ToMatrix(Transform) (Transformation|GetWorldTransform (Variables|Default|GetStaticMesh))) (Variables|PivotPainterInputs|GetOrigin_Extent) (Variables|Textures|GetTimestamp) (Variables|Textures|GetNormal%20Random) (Utilities|Time|GetTimeSeconds))
      (:then
        (Variables|Default|SetIsWorking true))
      (:Completed
        (Variables|Default|SetIsWorking false)
        ;[1 0.7666 0] Ray hit or not?
        (Utilities|FlowControl|Sequence
          (:then_0
            ;[1 0.02848 0] Disable hited spheres at ray hit
            (Utilities|DisableSphereCollisionatIndex (.Count (Utilities|Struct|BreakOutStruct _outstruct)) (.OutIndexes (Utilities|Struct|BreakOutStruct _outstruct))))
          (:then_1
            (Utilities|IsValid WeaponReference
              (:Is%20Valid
                (if (>= (.HitDistance (Utilities|Struct|BreakOutStruct _outstruct)) 0.0)
                  (Default|SphereHit WeaponReference self (.HitDistance (Utilities|Struct|BreakOutStruct _outstruct)))
                  (else
                    (Default|MissHit WeaponReference self)))))))))))

(event EventBeginPlay
  ;[0.009702 0.1927 0] Begin Play
  (if (Variables|PivotPainterInputs|GetSphere%20Collision%20Feedback)
    (CallFunction|ReadCollsionfromOriginTexture)
    (Utilities|SetupCollisionforMainMesh false)
    (Variables|Default|SetIsWorking false)
    (else
      (Utilities|SetupCollisionforMainMesh true))))

(fn ConstructionScript
  (bind _3d_mesh (Variables|PivotPainterInputs|Get3d%20Mesh))
  (Utilities|IsValid _3d_mesh
    (:Is%20Valid
      (Components|StaticMesh|SetStaticMesh (Variables|Default|GetStaticMesh) _3d_mesh)
      (CallFunction|InitializeTexturesandMaterials))))

(fn InitializeTexturesandMaterials
  (bind _origin_extent (Variables|PivotPainterInputs|GetOrigin_Extent))
  (bind _origin_extent_2 (Variables|PivotPainterInputs|GetOrigin_Extent))
  (Utilities|IsValid (Variables|PivotPainterInputs|GetOrigin_Extent)
    (:Is%20Valid
      (bind _returnvalue (Rendering|CreateRenderTarget2D (Class|Texture2D|BlueprintGetSizeX _origin_extent) (Class|Texture2D|BlueprintGetSizeY _origin_extent) "RTF_R32f" "(R=0.000000,G=0.000000,B=0.000000,A=1.000000)" false true))
      (Variables|/Script/Engine.Texture|SetLODGroup _returnvalue "TEXTUREGROUP_16BitData")
      (Variables|Textures|SetTimestamp _returnvalue)
      (bind _returnvalue_2 (Rendering|CreateRenderTarget2D (Class|Texture2D|BlueprintGetSizeX _origin_extent_2) (Class|Texture2D|BlueprintGetSizeY _origin_extent_2) "RTF_RGBA16f" "(R=0.000000,G=0.000000,B=0.000000,A=0.000000)" false true))
      (Variables|/Script/Engine.Texture|SetLODGroup _returnvalue_2 "TEXTUREGROUP_16BitData")
      (Variables|Textures|SetNormal%20Random _returnvalue_2)
      (for (_array_element _array_index) (Rendering|Material|GetMaterials (Variables|Default|GetStaticMesh))
        (bind _returnvalue_3 (Rendering|Material|CreateDynamicMaterialInstance _array_element "None" "None" :!class /Script/Engine.KismetMaterialLibrary))
        (Rendering|Material|SetTextureParameterValue _returnvalue_3 "Timestamp" (Variables|Textures|GetTimestamp))
        (Rendering|Material|SetTextureParameterValue _returnvalue_3 "Normal_Random" (Variables|Textures|GetNormal%20Random))
        (Rendering|Material|SetTextureParameterValue _returnvalue_3 "Origin_Extent" (Variables|PivotPainterInputs|GetOrigin_Extent))
        (Rendering|Material|SetMaterial (Variables|Default|GetStaticMesh) _array_index _returnvalue_3)))))

(fn ReadCollsionfromOriginTexture
  (bind _origin_extent (Variables|PivotPainterInputs|GetOrigin_Extent))
  (bind _origin_extent_2 (Variables|PivotPainterInputs|GetOrigin_Extent))
  (Utilities|IsValid (Variables|PivotPainterInputs|GetOrigin_Extent)
    (:Is%20Valid
      (bind _returnvalue (Rendering|CreateRenderTarget2D (Class|Texture2D|BlueprintGetSizeX _origin_extent) (Class|Texture2D|BlueprintGetSizeY _origin_extent) "RTF_RGBA16f" "(R=0.000000,G=0.000000,B=0.000000,A=0.000000)" false true))
      (bind _output_get (LocalVariables|SetOrigin_Extent_Copy _returnvalue))
      (Class|PivotPainterDestroyComputeLibraryAsyncExecution|CopyTexturetoRenderTarget (Variables|PivotPainterInputs|GetOrigin_Extent) _output_get)
      (Utilities|Map|Clear (Variables|Default|GetSphere%20Collision%20Array))
      (LocalVariables|SetElement%20Index 0)
      (for _index (range 0 (- (Class|Texture2D|BlueprintGetSizeY _origin_extent_2) 1))
        (for _index_2 (range 0 (- (Class|Texture2D|BlueprintGetSizeX _origin_extent_2) 1))
          (bind _returnvalue_2 (Class|KismetRenderingLibrary|ReadRenderTargetRawPixel (LocalVariables|GetOrigin_Extent_Copy) _index_2 _index false))
          (if (not (< (* (.A (Utilities|Struct|BreakLinearColor _returnvalue_2)) 0.01) 0.0001))
            (bind _returnvalue_3 (AddComponent|AddSphereComponent (Components|GetOwner (Variables|Default|GetStaticMesh)) false (Math|Transform|MakeTransform (Math|Vector|MakeVector (.R (Utilities|Struct|BreakLinearColor _returnvalue_2)) (.G (Utilities|Struct|BreakLinearColor _returnvalue_2)) (.B (Utilities|Struct|BreakLinearColor _returnvalue_2))) "0, 0, 0" (Math|Conversions|ToVector(Float) (* (.A (Utilities|Struct|BreakLinearColor _returnvalue_2)) 0.01)))))
            (Transformation|AttachComponentToComponent _returnvalue_3 (Variables|Default|GetStaticMesh) "None" "KeepRelative" "KeepRelative" "KeepRelative" false)
            (Utilities|SetupCollisionforSphere _returnvalue_3)
            (Utilities|Map|Add (Variables|Default|GetSphere%20Collision%20Array) (LocalVariables|GetElement%20Index) _returnvalue_3)
            (LocalVariables|SetElement%20Index (+ (LocalVariables|GetElement%20Index) 1))))))))